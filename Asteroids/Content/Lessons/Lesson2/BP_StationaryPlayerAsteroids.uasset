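; Stationary player for the Lesson 2 asteroids scene that targets flying asteroids by VR camera gaze.
; Each tick it places a material billboard far along the camera's forward vector as an aim marker, also running a line trace whose result is unused.
; Left mouse click line-traces on the Visibility channel along that gaze and calls Interact on any FlyingAsteroid hit.
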(event EventTick
  (params (DeltaSeconds :type Float%20%28single-precision%29))
  (bind (_location _forward_vector) (CallFunction|GetPlayerVRCameraProperties))
  (Collision|LineTraceByChannel _location (+ _location (* _forward_vector 1000000000)) "TraceTypeQuery1" false 0 "None")
  (Transformation|SetWorldLocation (Variables|Default|GetMaterialBillboard) (+ _location (* _forward_vector 1000000000)) false false))

(event EventBeginPlay)

(event Collision|EventActorBeginOverlap
  (params (OtherActor :type Actor%20Object%20Reference)))

(event Input|MouseEvents|LeftMouseButton
  (params (Key :type Key%20Structure :default "AnyKey"))
  (:Pressed
    (bind (_location _forward_vector) (CallFunction|GetPlayerVRCameraProperties))
    (bind (_outhit _returnvalue) (Collision|LineTraceByChannel _location (+ _location (* _forward_vector 1000000000)) "TraceTypeQuery1" false 0 "None"))
    (if _returnvalue
      (bind _asflying_asteroid (Utilities|Casting|CastToFlyingAsteroid (.HitActor (Collision|BreakHitResult _outhit))))
      (Default|Interact _asflying_asteroid))))

(fn ConstructionScript)